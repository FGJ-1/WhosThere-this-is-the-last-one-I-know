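; BP_DialogueObject is an interactable world object that steps through lines of dialogue and uses a configurable mesh.
; Each Interact plays a sound and advances the DialogueText array, creating the dialogue widget on the first line, updating it after, then removing it and resetting the index.
; Interaction functions supply type, location, prompt and timing; ShowObject reveals ToggledActor with a sound.
; Disconnected leftovers include a DataTable-driven dialogue chain and HideObject's hiding logic.
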(event EventBeginPlay)

(event EventInteract
  (params (Interactor :type Actor%20Object%20Reference))
  (Audio|PlaySoundatLocation (Variables|Default|GetSoundToPlay) (Transformation|GetActorLocation) "0, 0, 0" 1.0 1.0 0.0 0 0 0 0)
  (if (<= (Variables|Default|GetDialogueIndex) (Utilities|Array|LastIndex (Variables|Default|GetDialogueText)))
    (if (== (Variables|Default|GetDialogueIndex) 0)
      (bind _returnvalue (UserInterface|CreateWidget "/Game/Assets/Scripts/Dialogue/BP_DialogueWidget.BP_DialogueWidget_C" 0 (Variables|Default|GetDialogueName) (Utilities|Array|Get(acopy) (Variables|Default|GetDialogueText) (Variables|Default|GetDialogueIndex))))
      (bind _output_get (Variables|Default|SetDialogueWidget _returnvalue))
      (UserInterface|Viewport|AddtoViewport _output_get 0)
      (else
        (Default|UpdateDialogue (Variables|Default|GetDialogueWidget) (Utilities|Array|Get(acopy) (Variables|Default|GetDialogueText) (Variables|Default|GetDialogueIndex)))))
    (Math|Integer|IncrementInt (Variables|Default|GetDialogueIndex))
    (else
      (Widget|RemovefromParent (Variables|Default|GetDialogueWidget))
      (Variables|Default|SetDialogueIndex 0))))

(fn ConstructionScript
  (Components|StaticMesh|SetStaticMesh (Variables|Default|GetStaticMesh) (Variables|Default|GetItemModelToPlace)))

(fn HideObject)

(fn ShowObject
  (Audio|PlaySoundatLocation "/Engine/VREditor/Sounds/UI/Scaling_Up.Scaling_Up" (Transformation|GetActorLocation) "0, 0, 0" 1.0 1.0 0.0 0 0 0 0)
  (Rendering|SetActorHiddenInGame (Variables|Default|GetToggledActor) false))

(fn GetHoldDuration
  (return (Variables|Default|GetHoldDuration)))

(fn GetInteractionLocation
  (return (Transformation|GetWorldLocation (Variables|Default|GetInteractionLocation))))

(fn GetInteractionPrompt
  (return "to equip"))

(fn GetInteractionType
  (return (Variables|Default|GetInteractionType)))

(fn GetTapCount
  (return 4))

(fn PickUp
  (return true))