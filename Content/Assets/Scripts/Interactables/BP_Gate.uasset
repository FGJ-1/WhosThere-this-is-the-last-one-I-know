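; BP_Gate is an interactable gate that toggles open and closed when the player interacts with it.
; Interact flips IsOpen and plays or reverses a timeline that rotates the static mesh in yaw, printing a debug string.
; It answers interaction queries with a state-dependent prompt, a component's world location and fixed type, hold and tap settings, and refuses pickup.
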(event Custom|CloseDoor
  (Variables|Default|SetIsOpen false)
  (bind _zrotation (Timeline|OpenDoorTimeline Reverse)
    (:Update
      (Transformation|SetRelativeRotation (Variables|Default|GetStaticMesh) (Math|Rotator|MakeRotator 0.0 0.0 _zrotation) false false))))

(event Custom|OpenDoor
  (Variables|Default|SetIsOpen true)
  (bind _zrotation (Timeline|OpenDoorTimeline Play)
    (:Update
      (Transformation|SetRelativeRotation (Variables|Default|GetStaticMesh) (Math|Rotator|MakeRotator 0.0 0.0 _zrotation) false false))))

(event EventBeginPlay)

(event EventInteract
  (params (Interactor :type Actor%20Object%20Reference))
  (if (Variables|Default|GetIsOpen)
    (CallFunction|CloseDoor)
    (Development|PrintString "close")
    (else
      (CallFunction|OpenDoor)
      (Development|PrintString "Open"))))

(fn ConstructionScript)

(fn GetHoldDuration
  (return 0.0))

(fn GetInteractionLocation
  (return (Transformation|GetWorldLocation (Variables|Default|GetInteractionLocation))))

(fn GetInteractionPrompt
  (return (select (Variables|Default|GetIsOpen) "to close the door" "to open the door")))

(fn GetInteractionType
  (return "NewEnumerator0"))

(fn GetTapCount
  (return 4))

(fn PickUp
  (return false))