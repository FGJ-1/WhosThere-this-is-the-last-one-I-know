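; BP_PickUpItem1 is an interactable pickup actor that exposes interaction type, hold duration, tap count and a world-space interaction location through getter functions.
; Interact prints debug text claiming the item was added to the interactor's inventory, plays a sound at the actor's location, then destroys the actor.
; No inventory call is made: PickUp only returns false, the prompt is empty and the tap count is hardcoded.
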(event EventInteract
  (params (Interactor :type Actor%20Object%20Reference))
  (Development|PrintString "huh")
  (Development|PrintString (Utilities|String|ToString(Text) (Utilities|Text|FormatText "Added {itemName} to the inventory of {ActorName}" (Utilities|GetDisplayName self) (Utilities|GetDisplayName Interactor))))
  (Audio|PlaySoundatLocation 0 (Transformation|GetActorLocation) "0, 0, 0" 1.0 1.0 0.0 0 0 0 0)
  (Actor|DestroyActor))

(fn ConstructionScript)

(fn GetHoldDuration
  (return (Variables|Default|GetHoldDuration)))

(fn GetInteractionLocation
  (return (Transformation|GetWorldLocation (Variables|Default|GetInteractionLocation))))

(fn GetInteractionPrompt
  (return ""))

(fn GetInteractionType
  (return (Variables|Default|GetInteractionType)))

(fn GetTapCount
  (return 4))

(fn PickUp
  (return false))