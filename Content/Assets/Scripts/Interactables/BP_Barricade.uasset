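; BP_Barricade is an interactable barricade that starts invisible and appears when the player sets it up.
; BeginPlay hides the static mesh, and the first Interact shows it and latches IsSet, so later calls do nothing.
; Getter functions supply constant prompt, interaction type, tap count and hold settings, suggesting a repeated-tap interaction, and PickUp always returns false.
; Only visibility is toggled; collision is untouched.
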(event EventBeginPlay
  (Rendering|SetVisibility (Variables|Default|GetStaticMesh) false false))

(event Collision|EventActorBeginOverlap
  (params (OtherActor :type Actor%20Object%20Reference)))

(event EventInteract
  (params (Interactor :type Actor%20Object%20Reference))
  (if (not (Variables|Default|GetIsSet))
    (Rendering|SetVisibility (Variables|Default|GetStaticMesh) true false)
    (Variables|Default|SetIsSet true)))

(fn ConstructionScript)

(fn GetHoldDuration
  (return 0.0))

(fn GetInteractionLocation
  (return "0, 0, 0"))

(fn GetInteractionPrompt
  (return "barricade"))

(fn GetInteractionType
  (return "NewEnumerator2"))

(fn GetTapCount
  (return 8))

(fn PickUp
  (return false))