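; BP_HidingSpot is an interactable that toggles the player in and out of a hiding place, with a configurable mesh.
; Hiding attaches the player, moves them to an offset from InteractionLocation, flags InHidingSpot and disables capsule collision.
; Unhiding line-traces down and sideways, then detaches the player at the hit point, without re-enabling collision or clearing InHidingSpot.
; Interaction getters still return pickup-style values like "to equip".
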(event Custom|Hide
  (bind _playerref (Variables|Default|GetPlayerRef))
  (bind _interactionlocation (Variables|Default|GetInteractionLocation))
  (Transformation|AttachComponentToComponent (Variables|Default|GetPlayerRef) (Variables|Transformation|GetRootComponent) "None" "KeepRelative" "KeepRelative" "KeepRelative" true)
  (Transformation|SetActorTransform (Variables|Default|GetPlayerRef) (Math|Transform|MakeTransform (+ (Transformation|GetWorldLocation _interactionlocation) (Variables|Default|GetNewLocation)) (Math|Rotator|CombineRotators (Variables|Default|GetNewRotation) (Transformation|GetWorldRotation _interactionlocation)) "1.000000,1.000000,1.000000"))
  (bind _asbp_player (Utilities|Casting|CastToBP_Player _playerref))
  (Variables|/Game/Assets/Scripts/BP_Player.BP_Player_C|SetInHidingSpot _asbp_player true)
  (Variables|Default|SetIsHiding true)
  (Collision|SetCollisionEnabled (Actor|GetComponentbyClass _playerref "/Script/Engine.CapsuleComponent") "NoCollision"))

(event Custom|Unhide
  (bind _playerref (Variables|Default|GetPlayerRef))
  (bind _playerref_2 (Variables|Default|GetPlayerRef))
  (bind _returnvalue (Transformation|GetActorLocation _playerref_2))
  (bind (_outhit _returnvalue_2) (Collision|LineTraceByChannel _returnvalue (- _returnvalue "0.000000,-100.000000,500.000000") "TraceTypeQuery1" false 0 "None"))
  (if _returnvalue_2
    (Development|PrintString (Utilities|GetDisplayName (.HitActor (Collision|BreakHitResult _outhit))))
    (Transformation|DetachFromActor _playerref "KeepRelative" "KeepRelative" "KeepRelative")
    (Transformation|SetActorTransform _playerref (Math|Transform|MakeTransform (.Location (Collision|BreakHitResult _outhit)) "0, 0, 0" "1.000000,1.000000,1.000000"))
    (Variables|Default|SetIsHiding false)
    (for _array_element (Actor|GetComponentsbyTag _playerref "/Script/Engine.CapsuleComponent" "None")
      (Components|Activation|SetActive _array_element false false))
    (else
      (Development|PrintString "Missed"))))

(event Custom|UnhideMessage_Event
  (bind _playerref (Variables|Default|GetPlayerRef))
  (bind _playerref_2 (Variables|Default|GetPlayerRef))
  (bind _returnvalue (Transformation|GetActorLocation _playerref_2))
  (bind (_outhit _returnvalue_2) (Collision|LineTraceByChannel _returnvalue (- _returnvalue "0.000000,-100.000000,500.000000") "TraceTypeQuery1" false 0 "None"))
  (if _returnvalue_2
    (Development|PrintString (Utilities|GetDisplayName (.HitActor (Collision|BreakHitResult _outhit))))
    (Transformation|DetachFromActor _playerref "KeepRelative" "KeepRelative" "KeepRelative")
    (Transformation|SetActorTransform _playerref (Math|Transform|MakeTransform (.Location (Collision|BreakHitResult _outhit)) "0, 0, 0" "1.000000,1.000000,1.000000"))
    (Variables|Default|SetIsHiding false)
    (for _array_element (Actor|GetComponentsbyTag _playerref "/Script/Engine.CapsuleComponent" "None")
      (Components|Activation|SetActive _array_element false false))
    (else
      (Development|PrintString "Missed"))))

(event EventBeginPlay)

(event EventInteract
  (params (Interactor :type Actor%20Object%20Reference))
  (bind _asbp_player (Utilities|Casting|CastToBP_Player Interactor)
    (:then
      (bind _output_get (Variables|Default|SetBP_PlayerRef _asbp_player))
      (Variables|/Game/Assets/Scripts/BP_Player.BP_Player_C|SetOldLocation _output_get (Math|Conversions|ToTransform(Vector) (Transformation|GetWorldLocation (Variables|/Script/Engine.Actor|GetRootComponent (Variables|Default|GetBP_PlayerRef))))))
    (:CastFailed
      (Development|PrintString "wtf")))
  (Variables|Default|SetPlayerRef Interactor)
  (Audio|PlaySoundatLocation "/Engine/VREditor/Sounds/UI/Scaling_Up.Scaling_Up" (Transformation|GetActorLocation) "0, 0, 0" 1.0 1.0 0.0 0 0 0 0)
  (if (Variables|Default|GetIsHiding)
    (CallFunction|Unhide)
    (Development|PrintString "unhiding now")
    (else
      (CallFunction|Hide)
      (Development|PrintString "hiding now"))))

(fn ConstructionScript
  (Components|StaticMesh|SetStaticMesh (Variables|Default|GetStaticMesh) (Variables|Default|GetItemModelToPlace)))

(fn GetEquippable
  (return true))

(fn GetEquipped
  (return 0))

(fn GetHoldDuration
  (return (Variables|Default|GetHoldDuration)))

(fn GetInteractionLocation
  (return (Transformation|GetWorldLocation (Variables|Default|GetInteractionLocation))))

(fn GetInteractionPrompt
  (return "to equip"))

(fn GetInteractionType
  (return (Variables|Default|GetInteractionType)))

(fn GetTapCount
  (return 4))

(fn PickUp
  (return true))