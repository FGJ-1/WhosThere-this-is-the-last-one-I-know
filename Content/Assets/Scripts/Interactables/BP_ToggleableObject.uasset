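; Interactable object that shows or hides a referenced ToggledActor each time it is used.
; BeginPlay applies the initial IsToggled state, and Interact plays a sound, then flips that state and the actor's visibility.
; The construction script sets the object's mesh from ItemModelToPlace, while getter functions supply interaction type, prompt, location, hold duration and tap count.
; HideObject is an empty stub, and ShowObject is a separate reveal-with-sound function unused by Interact.
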(event EventBeginPlay
  (bind _toggledactor (Variables|Default|GetToggledActor))
  (if (Variables|Default|GetIsToggled)
    (Variables|Default|SetIsToggled true)
    (Rendering|SetActorHiddenInGame _toggledactor false)
    (else
      (Variables|Default|SetIsToggled false)
      (Rendering|SetActorHiddenInGame _toggledactor true))))

(event EventInteract
  (params (Interactor :type Actor%20Object%20Reference))
  (bind _toggledactor (Variables|Default|GetToggledActor))
  (Audio|PlaySoundatLocation (Variables|Default|GetSoundToPlay) (Transformation|GetActorLocation) "0, 0, 0" 1.0 1.0 0.0 0 0 0 0)
  (if (Variables|Default|GetIsToggled)
    (Variables|Default|SetIsToggled false)
    (Rendering|SetActorHiddenInGame _toggledactor true)
    (else
      (Variables|Default|SetIsToggled true)
      (Rendering|SetActorHiddenInGame _toggledactor false))))

(fn ConstructionScript
  (Components|StaticMesh|SetStaticMesh (Variables|Default|GetStaticMesh) (Variables|Default|GetItemModelToPlace)))

(fn HideObject)

(fn ShowObject
  (Audio|PlaySoundatLocation "/Engine/VREditor/Sounds/UI/Scaling_Up.Scaling_Up" (Transformation|GetActorLocation) "0, 0, 0" 1.0 1.0 0.0 0 0 0 0)
  (Rendering|SetActorHiddenInGame (Variables|Default|GetToggledActor) false))

(fn GetHoldDuration
  (return (Variables|Default|GetHoldDuration)))

(fn GetInteractionLocation
  (return (Transformation|GetWorldLocation (Variables|Default|GetInteractionLocation))))

(fn GetInteractionPrompt
  (return "to equip"))

(fn GetInteractionType
  (return (Variables|Default|GetInteractionType)))

(fn GetTapCount
  (return 4))

(fn PickUp
  (return true))