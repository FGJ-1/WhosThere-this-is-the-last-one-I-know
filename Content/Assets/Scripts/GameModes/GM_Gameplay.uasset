(event EventBeginPlay
  (Utilities|FlowControl|Sequence
    (:then_0
      (bind _returnvalue (UserInterface|CreateWidget "/Game/Assets/Scripts/HUDs/Gamemode_HUD.Gamemode_HUD_C"))
      (bind _output_get (Variables|Default|SetHUD _returnvalue))
      (UserInterface|Viewport|AddtoViewport _output_get 0)
      (Rendering|Components|TextRender|SetText (Variables|/Game/Assets/Scripts/HUDs/Gamemode_HUD.Gamemode_HUD_C|GetSurvivalText (Variables|Default|GetHUD)) "Investigate"))))

(event EventTick
  (params (DeltaSeconds :type Float%20%28single-precision%29))
  (switch Utilities|FlowControl|Switch|SwitchonE_GameState (Variables|Default|GetCurrentState)
    (:NewEnumerator0
      (CallFunction|UpdateGameTimer DeltaSeconds (Variables|Default|GetSetupTimeRemaining)))
    (:NewEnumerator1
      (CallFunction|UpdateGameTimer DeltaSeconds (Variables|Default|GetSurviveTimeRemaining)))
    (:NewEnumerator2
      (CallFunction|OutOfTime)
      (Utilities|FlowControl|Delay 3.0)
      (CallFunction|StartLoss :!label _label))
    (:NewEnumerator3
      (goto _label))))

(fn ConstructionScript)

(fn UpdateGameTimer
  (params (DeltaTime :type Float%20%28double-precision%29) (TimeRemaining :type Float%20%28double-precision%29))
  (bind _returnvalue (- TimeRemaining DeltaTime))
  (bind _hud (Variables|Default|GetHUD))
  (bind _timetext (Variables|/Game/Assets/Scripts/HUDs/Gamemode_HUD.Gamemode_HUD_C|GetTimeText _hud))
  (if (== (Variables|Default|GetCurrentState) 0)
    (bind _output_get (Variables|Default|SetSetupTimeRemaining _returnvalue))
    (bind _format_time (CallFunction|TimeRemainingFormat _output_get))
    (Rendering|Components|TextRender|SetText _timetext _format_time)
    (if (<= (Variables|Default|GetSetupTimeRemaining) 0.0)
      (CallFunction|StartSurvival))
    (else
      (bind _output_get_2 (Variables|Default|SetSurviveTimeRemaining _returnvalue))
      (bind _format_time_2 (CallFunction|TimeRemainingFormat _output_get_2))
      (Rendering|Components|TextRender|SetText _timetext _format_time_2)
      (if (<= (Variables|Default|GetSurviveTimeRemaining) 0.0)
        (CallFunction|OutOfTime)))))

(fn DisablePlayerInput
  (Input|DisableInput (Game|Player|GetPlayerPawn 0) 0))

(fn StartInvestigation
  (Variables|Default|SetCurrentState "NewEnumerator0")
  (Input|EnableInput (Game|Player|GetPlayerPawn 0) 0)
  (Rendering|Components|TextRender|SetText (Variables|/Game/Assets/Scripts/HUDs/Gamemode_HUD.Gamemode_HUD_C|GetTimeText (Variables|Default|GetHUD)) ""))

(fn OutOfTime
  (bind _hud (Variables|Default|GetHUD))
  (bind _survivaltext (Variables|/Game/Assets/Scripts/HUDs/Gamemode_HUD.Gamemode_HUD_C|GetSurvivalText _hud))
  (Variables|Default|SetCurrentState "NewEnumerator2")
  (Rendering|Components|TextRender|SetText (Variables|/Game/Assets/Scripts/HUDs/Gamemode_HUD.Gamemode_HUD_C|GetTimeText (Variables|Default|GetHUD)) "00:00")
  (CallFunction|DisablePlayerInput)
  (Rendering|Components|TextRender|SetText _survivaltext "You survived")
  (Widget|SetVisibility _survivaltext "Visible"))

(fn TimeRemainingFormat
  (params (TimeRemaining :type Float%20%28double-precision%29))
  (bind _returnvalue (/ TimeRemaining 6e+01))
  (bind _returnvalue_2 (Class|KismetMathLibrary|FFloor64 _returnvalue))
  (return (Utilities|Text|FormatText "{Minutes}:{Seconds}" (Utilities|Text|ToText(String) _returnvalue_2) (Utilities|Text|ToText(Float) (- TimeRemaining (* _returnvalue_2 60)) "HalfToEven" false true 2 324 0 0))))

(fn StartSurvival
  (bind _hud (Variables|Default|GetHUD))
  (bind _survivaltext (Variables|/Game/Assets/Scripts/HUDs/Gamemode_HUD.Gamemode_HUD_C|GetSurvivalText _hud))
  (Variables|Default|SetCurrentState "NewEnumerator1")
  (Rendering|Components|TextRender|SetText _survivaltext "Survive the night")
  (Widget|SetVisibility _survivaltext "Visible"))

(fn StartWin
  (Variables|Default|SetCurrentState "NewEnumerator4")
  (Widget|SetVisibility (Variables|Default|GetHUD) "Collapsed")
  (bind _returnvalue (UserInterface|CreateWidget "/Game/Assets/Scripts/HUDs/WB_WinScreen.WB_WinScreen_C"))
  (UserInterface|Viewport|AddtoViewport _returnvalue 0))

(fn StartLoss
  (Variables|Default|SetCurrentState "NewEnumerator3")
  (Widget|SetVisibility (Variables|Default|GetHUD) "Collapsed")
  (bind _returnvalue (UserInterface|CreateWidget "/Game/Assets/Scripts/HUDs/WB_Lose.WB_Lose_C"))
  (UserInterface|Viewport|AddtoViewport _returnvalue 0))

(fn UpdateWinText)